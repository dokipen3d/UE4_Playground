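; BP_DataStream is a spline-based data stream effect actor, built entirely in the Construction Script.
; It adds spline meshes with the data stream material between consecutive spline points, matching tangents and roll (offset 90 degrees) at a set width.
; The segment count comes from spline length divided by mesh size, not from the point count.
; Each segment also spawns particle systems at seeded random distances along the whole spline.
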(event `self.ReceiveBeginPlay`)

(event `self.ReceiveActorBeginOverlap`
  (params (OtherActor :type "Actor Object Reference")))

(event `self.ReceiveTick`
  (params (DeltaSeconds :type "Float (single-precision)")))

(fn `UserConstructionScript`
  (bind _spline (`self.Spline`))
  (bind _width (`self.width`))
  (bind _spline_2 (`self.Spline`))
  (bind _spline_3 (`self.Spline`))
  (bind _returnvalue (`KismetMathLibrary.MakeVector2D` _width _width))
  (`KismetArrayLibrary.Array_Clear` (`self.particleSystems`))
  (for _index (range (+ (- (`KismetMathLibrary.FFloor` (/ (`SplineComponent.GetSplineLength` _spline_3) (`self.meshSize`))) 2) 1))
    (bind _returnvalue_2 (`AddComponent|Spline Mesh Component_44` :`bManualAttachment` true :!label _label))
    (bind _returnvalue_3 (+ _index 1))
    (`SplineMeshComponent.SetStartAndEnd` _returnvalue_2 (`SplineComponent.GetLocationAtSplinePoint` _spline_3 _index "World") (`SplineComponent.GetTangentAtSplinePoint` _spline _index "World") (`SplineComponent.GetLocationAtSplinePoint` _spline_3 _returnvalue_3 "World") (`SplineComponent.GetTangentAtSplinePoint` _spline _returnvalue_3 "World"))
    (`SplineMeshComponent.SetStartScale` _returnvalue_2 _returnvalue)
    (`SplineMeshComponent.SetEndScale` _returnvalue_2 _returnvalue)
    (`SplineMeshComponent.SetStartRoll` _returnvalue_2 (* (+ (`SplineComponent.GetRollAtSplinePoint` _spline _index "World") 90.0) 0.017))
    (`SplineMeshComponent.SetEndRoll` _returnvalue_2 (* (+ (`SplineComponent.GetRollAtSplinePoint` _spline _returnvalue_3 "World") 90.0) 0.017))
    (`PrimitiveComponent.SetMaterial` _returnvalue_2 0 "/Game/DanContent/FX_DataStream/Material/M_DataStream.M_DataStream")
    (for _ (range (`self.numPart`))
      (bind _returnvalue_4 (`AddComponent|Particle System Component_0` :`bManualAttachment` true))
      (`SceneComponent.K2_SetWorldLocation` _returnvalue_4 (`SplineComponent.GetLocationAtDistanceAlongSpline` _spline_2 (* (`KismetMathLibrary.RandomFloatFromStream` (`self.randS`)) (`SplineComponent.GetSplineLength` _spline_2)) "World") false false)))
  (goto _label))