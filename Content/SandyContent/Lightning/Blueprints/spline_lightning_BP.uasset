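; Spline lightning actor Blueprint that builds a spline path between a start and an end position.
; The construction script appends StartPos, evenly stepped intermediate points and EndPos in local space, with NumberOfPoints setting the count.
; Intermediate points are multiples of the start-to-end step without the StartPos offset, and existing spline points are not cleared.
; It has no active event logic, visuals or randomised displacement.
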(event `self.ReceiveBeginPlay`)

(event `self.ReceiveActorBeginOverlap`
  (params (OtherActor :type "Actor Object Reference")))

(event `self.ReceiveTick`
  (params (DeltaSeconds :type "Float (single-precision)")))

(fn `UserConstructionScript`
  (bind _startpos (`self.startPos`))
  (bind _endpos (`self.endPos`))
  (bind _spline (`self.Spline`))
  (bind _returnvalue (- (`self.numberOfPoints`) 2))
  (`SplineComponent.AddSplinePoint` _spline _startpos "Local")
  (for _index (range 1 (+ _returnvalue 1))
    (`SplineComponent.AddSplinePoint` _spline (* (/ (- _endpos _startpos) (`KismetMathLibrary.Conv_IntToDouble` _returnvalue)) _index) "Local"))
  (`SplineComponent.AddSplinePoint` _spline _endpos "Local"))