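; Lightning bolt effect actor that builds a bolt between StartPos and EndPos and animates it on FireBolt.
; The construction script builds a spline with seeded noise on interior points.
; Each segment gets a seeded-random lightning spline mesh plus a fixed gap-filler mesh, using two separate dynamic materials.
; FireBolt plays a timeline driving each material's reveal radius from the start point, plus shared glow and fade.
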(event `self.ReceiveBeginPlay`)

(event `self.ReceiveActorBeginOverlap`
  (params (OtherActor :type "Actor Object Reference")))

(event `self.ReceiveTick`
  (params (DeltaSeconds :type "Float (single-precision)")))

(event `FireBolt`
  (bind _boltmaterial (`self.boltMaterial`))
  (bind _branchmaterial (`self.branchMaterial`))
  (bind _emissivestrength (`self.EmissiveStrength`))
  (bind _fadeout (`self.FadeOut`))
  (bind _colour (`self.Colour`))
  (bind _returnvalue (`KismetMathLibrary.Conv_VectorToLinearColor` (+ (`self.K2_GetActorLocation`) (`self.startPos`))))
  (bind (_direction _revealbolt _revealbranching _gain _fade) (`Timeline|RevealBoltAndBranching_anim` :!via `PlayFromStart`)
    (:`Update`
      (set `self.RevealBolt` _revealbolt)
      (set `self.RevealBranching` _revealbranching)
      (set `self.EmissiveStrength` _gain)
      (set `self.FadeOut` _fade)
      ;[1 1 1] Drive Material Attributes
      (`MaterialInstanceDynamic.SetVectorParameterValue` _boltmaterial "PrimeLocation" _returnvalue)
      (`MaterialInstanceDynamic.SetScalarParameterValue` _boltmaterial "Radius" (`self.RevealBranching`))
      (`MaterialInstanceDynamic.SetScalarParameterValue` _boltmaterial "Gain" _emissivestrength)
      (`MaterialInstanceDynamic.SetVectorParameterValue` _boltmaterial "EmissiveColour" _colour)
      (`MaterialInstanceDynamic.SetScalarParameterValue` _boltmaterial "Fade" _fadeout)
      ;[1 1 1] Drive Material Attributes
      (`MaterialInstanceDynamic.SetVectorParameterValue` _branchmaterial "PrimeLocation" _returnvalue)
      (`MaterialInstanceDynamic.SetScalarParameterValue` _branchmaterial "Radius" (`self.RevealBolt`))
      (`MaterialInstanceDynamic.SetScalarParameterValue` _branchmaterial "Gain" _emissivestrength)
      (`MaterialInstanceDynamic.SetVectorParameterValue` _branchmaterial "EmissiveColour" _colour)
      (`MaterialInstanceDynamic.SetScalarParameterValue` _branchmaterial "Fade" _fadeout))))

(fn `UserConstructionScript`
  (bind _meshlist (`self.meshList`))
  (bind _seed (`self.seed`))
  (bind _spline (`self.Spline`))
  (bind _scene (`self.Scene`))
  (bind _boltmaterial (`self.boltMaterial`))
  (bind _branchmaterial (`self.branchMaterial`))
  (bind _numberofpoints (`self.numberOfPoints`))
  (bind _endpos (`self.endPos`))
  (bind _spline_2 (`self.Spline`))
  (bind _startpos (`self.startPos`))
  (bind _noisestrength (`self.noiseStrength`))
  (bind _emissivestrength (`self.EmissiveStrength`))
  (bind _colour (`self.Colour`))
  (bind _returnvalue (`KismetMathLibrary.Conv_VectorToLinearColor` (+ (`self.K2_GetActorLocation`) (`self.startPos`))))
  (`|ExecutionSequence`
    (:`then_0`
      ;[1 1 1] Build Main Spline and add any noise
      (`SplineComponent.ClearSplinePoints` _spline_2)
      (`SplineComponent.AddSplinePoint` _spline_2 _startpos "Local") ; Add start point with no noise
      (for _index (range 1 _numberofpoints)
        (`SplineComponent.AddSplinePoint` _spline_2 (`KismetMathLibrary.MakeVector` (+ (.x (* (/ (- _endpos _startpos) (`KismetMathLibrary.Conv_IntToDouble` _numberofpoints)) _index)) (`KismetMathLibrary.RandomFloatInRangeFromStream` 0.0 _noisestrength (`KismetMathLibrary.MakeRandomStream` (+ _seed 1 _index)))) (+ (.y (* (/ (- _endpos _startpos) (`KismetMathLibrary.Conv_IntToDouble` _numberofpoints)) _index)) (`KismetMathLibrary.RandomFloatInRangeFromStream` 0.0 _noisestrength (`KismetMathLibrary.MakeRandomStream` (+ _seed 2 _index)))) (+ (.z (* (/ (- _endpos _startpos) (`KismetMathLibrary.Conv_IntToDouble` _numberofpoints)) _index)) (`KismetMathLibrary.RandomFloatInRangeFromStream` 0.0 _noisestrength (`KismetMathLibrary.MakeRandomStream` (+ _seed 3 _index))))) "Local"))
      (`SplineComponent.AddSplinePoint` _spline_2 _endpos "Local") ; Add end point with no noise
      ;[1 1 1] List of Meshes to pick from
      (set `self.meshList` (`|MakeArray` "/Game/SandyContent/FX_Lightning/Meshes/SM_lightningBolt_f001.SM_lightningBolt_f001" "/Game/SandyContent/FX_Lightning/Meshes/SM_lightningBolt_f003.SM_lightningBolt_f003" "/Game/SandyContent/FX_Lightning/Meshes/SM_lightningBolt_f017.SM_lightningBolt_f017" "/Game/SandyContent/FX_Lightning/Meshes/SM_lightningBolt_f037.SM_lightningBolt_f037" "/Game/SandyContent/FX_Lightning/Meshes/SM_lightningBolt_f055.SM_lightningBolt_f055" "/Game/SandyContent/FX_Lightning/Meshes/SM_lightningBolt_f067.SM_lightningBolt_f067" "/Game/SandyContent/FX_Lightning/Meshes/SM_lightningBolt_f110.SM_lightningBolt_f110" "/Game/SandyContent/FX_Lightning/Meshes/SM_lightningBolt_f119.SM_lightningBolt_f119" "/Game/SandyContent/FX_Lightning/Meshes/SM_lightningBolt_f140.SM_lightningBolt_f140" "/Game/SandyContent/FX_Lightning/Meshes/SM_lightningBolt_f161.SM_lightningBolt_f161" "/Game/SandyContent/FX_Lightning/Meshes/SM_lightningBolt_f215.SM_lightningBolt_f215" "/Game/SandyContent/FX_Lightning/Meshes/SM_lightningBolt_f218.SM_lightningBolt_f218" "/Game/SandyContent/FX_Lightning/Meshes/SM_lightningBolt_f221.SM_lightningBolt_f221" "/Game/SandyContent/FX_Lightning/Meshes/SM_lightningBolt_f224.SM_lightningBolt_f224" "/Game/SandyContent/FX_Lightning/Meshes/SM_lightningBolt_f227.SM_lightningBolt_f227" "/Game/SandyContent/FX_Lightning/Meshes/SM_lightningBolt_f230.SM_lightningBolt_f230" :!type "StaticMesh Object Reference"))
      ;[1 1 1] Make material instances
      (bind _returnvalue_2 (`KismetMaterialLibrary.CreateDynamicMaterialInstance` "/Game/SandyContent/Masters/solid_emissive_material.solid_emissive_material")) ; make a material instance for the main bolt
      (set `self.boltMaterial` _returnvalue_2)
      (bind _returnvalue_3 (`KismetMaterialLibrary.CreateDynamicMaterialInstance` "/Game/SandyContent/Masters/solid_emissive_material.solid_emissive_material")) ; make a material instance for the branching
      (set `self.branchMaterial` _returnvalue_3)
      ;[1 1 1] Drive Material Attributes
      (`MaterialInstanceDynamic.SetVectorParameterValue` _boltmaterial "PrimeLocation" _returnvalue)
      (`MaterialInstanceDynamic.SetScalarParameterValue` _boltmaterial "Radius" (`self.RevealBranching`))
      (`MaterialInstanceDynamic.SetScalarParameterValue` _boltmaterial "Gain" _emissivestrength)
      (`MaterialInstanceDynamic.SetVectorParameterValue` _boltmaterial "EmissiveColour" _colour)
      ;[1 1 1] Drive Material Attributes
      (`MaterialInstanceDynamic.SetVectorParameterValue` _branchmaterial "PrimeLocation" _returnvalue)
      (`MaterialInstanceDynamic.SetScalarParameterValue` _branchmaterial "Radius" (`self.RevealBolt`))
      (`MaterialInstanceDynamic.SetScalarParameterValue` _branchmaterial "Gain" _emissivestrength)
      (`MaterialInstanceDynamic.SetVectorParameterValue` _branchmaterial "EmissiveColour" _colour)
      ;[1 1 1] Add a randomly picked spline Mesh component fitted to the master curve between each pair of points
      (for _index_2 (range (+ (- (`SplineComponent.GetNumberOfSplinePoints` (`self.Spline`)) 2) 1))
        (bind _returnvalue_4 (`AddComponent|SplineMeshComponent_960` :`bManualAttachment` true))
        (`StaticMeshComponent.SetStaticMesh` _returnvalue_4 (`KismetArrayLibrary.Array_Get` _meshlist (`KismetMathLibrary.RandomIntegerInRangeFromStream` 0 (`KismetArrayLibrary.Array_LastIndex` _meshlist) (`KismetMathLibrary.MakeRandomStream` (+ (`self.seed`) _index_2)))))
        (`PrimitiveComponent.SetMaterial` _returnvalue_4 0 (`self.boltMaterial`))
        (`SceneComponent.K2_AttachTo` _returnvalue_4 _scene "None" "KeepRelativeOffset" true)
        (bind (_location _tangent) (`SplineComponent.GetLocationAndTangentAtSplinePoint` _spline _index_2 "Local"))
        (bind (_location_2 _tangent_2) (`SplineComponent.GetLocationAndTangentAtSplinePoint` _spline (+ _index_2 1) "Local"))
        (`SplineMeshComponent.SetStartAndEnd` _returnvalue_4 _location _tangent _location_2 _tangent_2)
        ;[1 1 1] Add an extra single segment mesh to fill the gaps because of the way the meshes git fit to the segments
        (bind _returnvalue_5 (`AddComponent|SplineMeshComponent_288706` :`bManualAttachment` true))
        (`StaticMeshComponent.SetStaticMesh` _returnvalue_5 "/Game/SandyContent/FX_Lightning/Meshes/SM_lightningBolt_f227.SM_lightningBolt_f227")
        (`PrimitiveComponent.SetMaterial` _returnvalue_5 0 (`self.branchMaterial`))
        (`SceneComponent.K2_AttachTo` _returnvalue_5 _scene "None" "KeepRelativeOffset" true)
        (`SplineMeshComponent.SetStartAndEnd` _returnvalue_5 _location _tangent _location_2 _tangent_2)))))